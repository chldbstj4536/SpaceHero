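; BP_Gun is an automatic gun actor that periodically fires bursts of Bullet actors.
; Tick counts down a fire-rate timer, carrying over the remainder, then resets the burst count and calls Fire.
; Fire spawns a bullet at the gun's transform; for No Trace bullets it sets direction from FireDirection's forward vector and re-calls itself by timer until the burst ends.
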(event `self.ReceiveTick`
  (params (DeltaSeconds :type "Float (single-precision)"))
  (bind _output_get (set `self.FireRemainTime` (- (`self.FireRemainTime`) DeltaSeconds)))
  (if (<= _output_get 0.0)
    (set `self.FireRemainTime` (+ (`self.FireRemainTime`) (`self.FireRate`)))
    (set `self.RemainBullet` (`self.BurstFireCount`))
    (`self.Fire`)))

(fn `Fire`
  (bind _returnvalue (`|SpawnActorFromClass` (`self.Bullet`) (`self.GetTransform`) "AlwaysSpawn" "MultiplyWithRoot" null null))
  (`/Engine/EditorBlueprintResources/StandardMacros.DecrementInt` (`self.RemainBullet`)
    (:`  `
      (switch `/Game/Blueprints/ETraceType` (`/Game/Blueprints/BP_Object.TraceType` _returnvalue)
        (:`NewEnumerator0`
          (set `/Game/Blueprints/BP_Object.Direction` (`SceneComponent.GetForwardVector` (`self.FireDirection`)) _returnvalue)
          (if (> (`self.RemainBullet`) 0)
            (`KismetSystemLibrary.K2_SetTimer` null "Fire" (`self.BurstFireRate`))))))))

(fn `UserConstructionScript`)