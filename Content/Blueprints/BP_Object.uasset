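; BP_Object is an actor that moves in a straight line or homes in on a target, depending on its TraceType.
; On BeginPlay, both tracing modes pick a random actor of a class as Target and store the normalized direction toward it.
; Each tick it offsets itself along Direction by Speed without sweeping, and Always Trace re-aims at Target first.
; No Trace keeps its preset Direction, normalized at start.
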(event `self.ReceiveBeginPlay`
  (switch `/Game/Blueprints/ETraceType` (`self.TraceType`)
    (:`NewEnumerator0`
      _)
    (:`NewEnumerator1`
      (bind _outactors (`GameplayStatics.GetAllActorsOfClass` null :!label _label))
      (bind _output_get (set `self.Target` (`KismetArrayLibrary.Array_Random` _outactors)))
      (set `self.Direction` (- (`self.K2_GetActorLocation` _output_get) (`self.K2_GetActorLocation`))))
    (:`NewEnumerator2`
      (goto _label)))
  (set `self.Direction` (`KismetMathLibrary.Normal` (`self.Direction`))))

(event `self.ReceiveTick`
  (params (DeltaSeconds :type "Float (single-precision)"))
  (`self.SetDirection`)
  (`self.Move` DeltaSeconds))

(fn `Move`
  (params (DeltaTime :type "Float (double-precision)"))
  (`self.K2_AddActorWorldOffset` (* (* DeltaTime (`self.Speed`)) (`self.Direction`))))

(fn `SetDirection`
  (switch `/Game/Blueprints/ETraceType` (`self.TraceType`)
    (:`NewEnumerator2`
      (set `self.Direction` (`KismetMathLibrary.Normal` (- (`self.K2_GetActorLocation` (`self.Target`)) (`self.K2_GetActorLocation`)))))))

(fn `UserConstructionScript`)